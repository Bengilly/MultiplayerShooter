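; Invisibility powerup ability that hides the skeletal mesh of the player it is applied to until it expires.
; Activation stores the player and mesh component and hides the mesh in game; expiry unhides it if the player is still valid.
; A replicated state-change event sets the stored mesh and its children hidden to match the invisibility flag, with debug prints in each event.
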(event EventOnAbilityStateChanged
  (params (bIsInvisible :type Boolean))
  ;[1 1 1] On Replicated
  (Development|PrintString (Utilities|String|Append "IsInvisble = " (Utilities|String|ToString(Boolean) bIsInvisible)))
  (Development|SetHiddeninGame (Variables|Components|GetMeshComp) bIsInvisible true))

(event EventOnAbilityExpired
  (bind _powerupappliedto (Variables|Default|GetPowerupAppliedTo))
  ;[1 1 1] Expired
  (Development|PrintString "Ability expired")
  (Utilities|IsValid _powerupappliedto
    (:Is%20Valid
      (Development|SetHiddeninGame (Actor|GetComponentbyClass _powerupappliedto "/Script/Engine.SkeletalMeshComponent") false (Variables|Default|GetbPropagateToChildren)))))

(event EventOnAbilityActivated
  (params (PlayerToApplyPowerup :type Actor%20Object%20Reference))
  ;[1 1 1] Activated
  (Development|PrintString "Ability activated")
  (bind _output_get (Variables|Default|SetPowerupAppliedTo PlayerToApplyPowerup))
  (Development|PrintString (Utilities|GetDisplayName _output_get))
  (bind _output_get_2 (Variables|Components|SetMeshComp (Actor|GetComponentbyClass _output_get "/Script/Engine.SkeletalMeshComponent")))
  (Development|SetHiddeninGame _output_get_2 true (Variables|Default|GetbPropagateToChildren)))

(fn ConstructionScript)