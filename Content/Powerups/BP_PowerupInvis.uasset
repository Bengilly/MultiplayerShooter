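; BP_PowerupInvis is a powerup that makes the player it is applied to invisible until it expires.
; On activation, the authority stores the player, hides the pickup mesh and the player's skeletal mesh, and sets Invisible.
; On expiry, it unhides that skeletal mesh and clears the flag if the player is still valid.
; A RepNotify on Invisible calls InvisStateChanged to toggle the stored mesh's hidden state, including its children.
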(event EventOnExpired
  (bind _powerupappliedto (Variables|Default|GetPowerupAppliedTo))
  ;[1 1 1] Expired
  (Networking|SwitchHasAuthority
    (:Authority
      (Utilities|IsValid _powerupappliedto
        (:Is%20Valid
          (Development|SetHiddeninGame (Actor|GetComponentbyClass _powerupappliedto "/Script/Engine.SkeletalMeshComponent") false (Variables|Default|GetbPropagateToChildren))
          (Variables|Default|SetbInvisible false))))))

(event EventOnActivated
  (params (PlayerToApplyPowerup :type Actor%20Object%20Reference))
  ;[1 1 1] Activated
  (Networking|SwitchHasAuthority
    (:Authority
      (bind _output_get (Variables|Default|SetPowerupAppliedTo PlayerToApplyPowerup))
      (Rendering|SetVisibility (Variables|Default|GetMeshComponent) false false)
      (bind _output_get_2 (Variables|Default|SetMeshComp (Actor|GetComponentbyClass _output_get "/Script/Engine.SkeletalMeshComponent")))
      (Development|SetHiddeninGame _output_get_2 true (Variables|Default|GetbPropagateToChildren))
      (Variables|Default|SetbInvisible true))))

(fn ConstructionScript)

(fn OnRepBInvisible
  (CallFunction|InvisStateChanged (Variables|Default|GetbInvisible)))

(fn InvisStateChanged
  (params (bInvisible :type Boolean))
  (bind _meshcomp (Variables|Default|GetMeshComp))
  (if bInvisible
    (Development|SetHiddeninGame _meshcomp true true)
    (else
      (Development|SetHiddeninGame _meshcomp false true))))