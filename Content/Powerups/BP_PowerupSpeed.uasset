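; Speed powerup actor that temporarily doubles the walk speed of the player it is applied to.
; On activation it stores that player, hides its mesh and sets MaxWalkSpeed to twice the movement component's current GetMaxSpeed.
; On expiry it sets MaxWalkSpeed to half the current GetMaxSpeed if the player is still valid, then destroys itself.
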(event EventOnExpired
  (bind _powerupappliedto (Variables|Default|GetPowerupAppliedTo))
  (bind _returnvalue (Actor|GetComponentbyClass _powerupappliedto "/Script/Engine.CharacterMovementComponent"))
  ;[1 1 1] Expired
  (Utilities|IsValid _powerupappliedto
    (:Is%20Valid
      (Variables|/Script/Engine.CharacterMovementComponent|SetMaxWalkSpeed _returnvalue (/ (Class|MovementComponent|GetMaxSpeed _returnvalue) 2.0)))
    (:Is%20Not%20Valid
      _))
  (Actor|DestroyActor))

(event EventOnActivated
  (params (PlayerToApplyPowerup :type Actor%20Object%20Reference))
  ;[1 1 1] Activated
  (bind _output_get (Variables|Default|SetPowerupAppliedTo PlayerToApplyPowerup))
  (Rendering|SetVisibility (Variables|Default|GetMeshComponent) false false)
  (Variables|/Script/Engine.CharacterMovementComponent|SetMaxWalkSpeed (Actor|GetComponentbyClass _output_get "/Script/Engine.CharacterMovementComponent") (* (Class|MovementComponent|GetMaxSpeed (Actor|GetComponentbyClass _output_get "/Script/Engine.CharacterMovementComponent")) 2.0)))

(fn ConstructionScript)