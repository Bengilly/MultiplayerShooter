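; Invisibility powerup pickup Blueprint whose Activated and Expired events are currently empty, so it adds no invisibility behavior of its own.
; Disconnected nodes retain an earlier approach that hides the pickup mesh, toggles the affected player's skeletal mesh and sets an Invisible flag.
; The OLD-suffixed state-change and RepNotify functions are also empty, with their visibility, destroy and debug-print nodes left unwired.
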(event EventOnExpired
  ;[1 1 1] Expired
)

(event EventOnActivated
  (params (PlayerToApplyPowerup :type Actor%20Object%20Reference))
  ;[1 1 1] Activated
)

(fn ConstructionScript)

(fn InvisStateChangedOLD
  (params (bInvisible :type Boolean)))

(fn OnRepBInvisibleOLD)