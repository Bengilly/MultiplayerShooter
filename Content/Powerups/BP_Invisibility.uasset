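; BP_Invisibility is a powerup that makes the player who receives it invisible until it expires.
; On activation it stores that player and hides their skeletal mesh component in game.
; On expiry it prints a debug message and, if the player is still valid, unhides the mesh.
; A separate state-change event sets the mesh's hidden state from an invisibility flag, propagating it to child components.
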(event EventOnActivated
  (params (PlayerToApplyPowerup :type Actor%20Object%20Reference))
  ;[1 1 1] Activated
  (bind _output_get (Variables|Default|SetPowerupAppliedTo PlayerToApplyPowerup))
  (bind _output_get_2 (Variables|Components|SetMeshComp (Actor|GetComponentbyClass _output_get "/Script/Engine.SkeletalMeshComponent")))
  (Development|SetHiddeninGame _output_get_2 true (Variables|Default|GetbPropagateToChildren)))

(event EventOnExpired
  (bind _powerupappliedto (Variables|Default|GetPowerupAppliedTo))
  ;[1 1 1] Expired
  (Development|PrintString "Ability expired")
  (Utilities|IsValid _powerupappliedto
    (:Is%20Valid
      (Development|SetHiddeninGame (Actor|GetComponentbyClass _powerupappliedto "/Script/Engine.SkeletalMeshComponent") false (Variables|Default|GetbPropagateToChildren)))))

(event EventOnAbilityStateChanged
  (params (bIsInvisible :type Boolean))
  (Development|SetHiddeninGame (Variables|Components|GetMeshComp) bIsInvisible true))

(fn ConstructionScript)