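; Behavior tree service that selects the nearest living player character as the AI pawn's target.
; Each tick it scans the actors known to the pawn's AI Perception sight sense, keeping BP_Character instances with health above zero.
; The closest one within a large distance cap is written to the TargetActorKey blackboard entry, which is set to None when no candidate qualifies.
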(event EventReceiveTickAI
  (params (OwnerController :type AI%20Controller%20Object%20Reference) (ControlledPawn :type Pawn%20Object%20Reference) (DeltaSeconds :type Float%20%28single-precision%29))
  (Variables|Default|SetClosestTargetActor 0)
  (Variables|Default|SetClosestTargetDistance 1e+05)
  (for _array_element (Class|AIPerceptionComponent|GetKnownPerceivedActors (Actor|GetComponentbyClass ControlledPawn "/Script/AIModule.AIPerceptionComponent") "/Script/AIModule.AISense_Sight")
    (if (Class|GameplayStatics|ObjectIsA _array_element "/Game/Blueprints/Player/BP_Character.BP_Character_C")
      (if (> (Variables|/Script/Shooter.SHealthComponent|GetCurrentHealth (Actor|GetComponentbyClass _array_element "/Script/Shooter.SHealthComponent")) 0.0)
        (if (< (Math|Vector|VectorLength (- (Transformation|GetActorLocation ControlledPawn) (Transformation|GetActorLocation _array_element))) (Variables|Default|GetClosestTargetDistance))
          (Variables|Default|SetClosestTargetDistance (Math|Vector|VectorLength (- (Transformation|GetActorLocation ControlledPawn) (Transformation|GetActorLocation _array_element))))
          (Variables|Default|SetClosestTargetActor _array_element)))))
  (Class|BTFunctionLibrary|SetBlackboardValueasObject (Variables|Default|GetTargetActorKey) (Variables|Default|GetClosestTargetActor)))