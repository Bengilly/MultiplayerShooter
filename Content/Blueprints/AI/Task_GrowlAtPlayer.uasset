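; Behavior tree task that makes a wolf AI growl at the player and marks it as chasing.
; On authority it multicasts an event that attaches a quiet, attenuated growl sound to the SWolf mesh and stores the audio component.
; The event sets HasGrowled and IsChasing on the wolf and finishes, or aborts if the cast fails.
; The HasGrowled check gates nothing, and the blackboard write is disconnected.
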(event Custom|Multicast_GrowlAtPlayer
  (params (ControlledPawn :type Pawn%20Object%20Reference))
  (bind _asswolf (Utilities|Casting|CastToSWolf ControlledPawn)
    (:then
      (if (Variables|/Script/Shooter.SWolf|GetbHasGrowled _asswolf)
        _
        (else
          _))
      (bind _returnvalue (Audio|SpawnSoundAttached "/Game/Sound/Wolf/WolfGrowling.WolfGrowling" (Variables|/Script/Engine.Character|GetMesh _asswolf) "None" "0, 0, 0" "0, 0, 0" "KeepRelativeOffset" false 0.1 1.0 0.0 "/Game/Sound/Wolf/SA_WolfGrowl.SA_WolfGrowl" 0))
      (Variables|/Script/Shooter.SWolf|SetWolfAudioComponent _asswolf _returnvalue)
      (Variables|/Script/Shooter.SWolf|SetbHasGrowled _asswolf true)
      (Variables|/Script/Shooter.SWolf|SetbIsChasing _asswolf true)
      (AI|BehaviorTree|FinishExecute true))
    (:CastFailed
      (Class|BTTaskBlueprintBase|FinishAbort))))

(event EventReceiveExecuteAI
  (params (OwnerController :type AI%20Controller%20Object%20Reference) (ControlledPawn :type Pawn%20Object%20Reference))
  (if (Ability|HasAuthority ControlledPawn)
    (CallFunction|MulticastGrowlatPlayer ControlledPawn)))