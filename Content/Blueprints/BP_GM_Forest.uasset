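; Forest game mode Blueprint that awards score for kills and contains enemy-spawning logic.
; On actor killed, a non-player pawn victim adds fixed points to the killer's SPlayerState and prints the score.
; An EQS result handler spawns BP_RollingDrone with debug spheres at returned locations, but the query is disconnected and SpawnEnemy is empty, so spawning never runs.
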(event Custom|OnQueryFinishedEvent_Event
  (params (QueryInstance :type Env%20Query%20Instance%20Blueprint%20Wrapper%20Object%20Reference) (QueryStatus :type EEnvQueryStatus%20Enum :default "Processing"))
  ;[1 1 1] Once query has finished, get results and spawn enemy in location
  (switch Utilities|FlowControl|Switch|SwitchonEEnvQueryStatus QueryStatus
    (:Success
      (bind _resultlocations (AI|EQS|GetQueryResultsasLocations QueryInstance))
      (for _array_element _resultlocations
        (Rendering|Debug|DrawDebugSphere _array_element 1e+02 12 "(R=0.484375,G=0.152777,B=0.000000,A=1.000000)" 3.0 2.0)
        (Game|SpawnActorfromClass "/Game/RollingDrone/BP_RollingDrone.BP_RollingDrone_C" (Math|Transform|MakeTransform _array_element) "AdjustIfPossibleButDontSpawnIfColliding" "MultiplyWithRoot" 0 0)))))

(event Custom|OnActorKilled_Event
  (params (EnemyKilled :type Actor%20Object%20Reference) (DamagingActor :type Actor%20Object%20Reference) (DamagingActorController :type Controller%20Object%20Reference))
  ;[1 1 1] Check if actor killed is a player pawn, if not, update player score
  (bind _aspawn (Utilities|Casting|CastToPawn EnemyKilled))
  (if (not (Pawn|IsPlayerControlled _aspawn))
    (bind _assplayer_state (Utilities|Casting|CastToSPlayerState (Variables|/Script/Engine.Pawn|GetPlayerState (Pawn|GetControlledPawn DamagingActorController))))
    (Class|SPlayerState|UpdateScore _assplayer_state 1e+01)
    (Development|PrintString (Utilities|String|ToString(Float) (Variables|/Script/Engine.PlayerState|GetScore _assplayer_state)) true true "(R=0.028321,G=1.000000,B=0.000000,A=1.000000)")))

(event EventSpawnEnemy)

(event EventBeginPlay
  (EventDispatchers|AssignOnActorKilled (delegate Custom|OnActorKilled_Event)))

(fn ConstructionScript)