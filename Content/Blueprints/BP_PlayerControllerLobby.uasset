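; Player controller for the multiplayer lobby that drives each client's lobby UI.
; On BeginPlay the local controller shows the mouse cursor and switches to UI-only input.
; Client-side events create and display the lobby and loading screen widgets.
; Another event clears and refills the lobby's player name list from the passed profile structs.
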(event EventShowLobbyMenu
  ;[1 1 1] Client - Load lobby widget
  (bind _returnvalue (UserInterface|CreateWidget "/Game/UI/Menus/WBP_Lobby.WBP_Lobby_C" self))
  (bind _output_get (Variables|Default|SetWBP_LobbyMenu _returnvalue))
  (UserInterface|Viewport|AddtoViewport _output_get 0))

(event EventBeginPlay
  ;[1 1 1] Set input mode to UI only on the local player controller
  (if (Pawn|IsLocalController)
    (Variables|Default|SetbShowMouseCursor true)
    (Input|SetInputModeUIOnly self 0 "DoNotLock" false)))

(event EventUpdatePlayerNames
  (params (AllPlayerProfileStructs :type Array%20of%20S%20Player%20Profile%20Struct%20Structures))
  (bind _wbp_lobbymenu (Variables|Default|GetWBP_LobbyMenu))
  ;[1 1 1] Client - Update player names on client UI
  (Utilities|IsValid _wbp_lobbymenu
    (:Is%20Valid
      (Default|ClearPlayerNames _wbp_lobbymenu)
      (Default|UpdatePlayerNames _wbp_lobbymenu AllPlayerProfileStructs))))

(event EventShowLoadingScreen
  ;[1 1 1] Client - Show loading screen widget
  (bind _returnvalue (UserInterface|CreateWidget "/Game/UI/Menus/WBP_LoadingScreen.WBP_LoadingScreen_C" self))
  (bind _output_get (Variables|Default|SetWBP_LoadScreen _returnvalue))
  (UserInterface|Viewport|AddtoViewport _output_get 0))

(fn ConstructionScript)