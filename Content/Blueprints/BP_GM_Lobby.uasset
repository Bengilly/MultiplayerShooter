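; Lobby game mode whose event graph is currently inert: the new-player and old lobby-update events have no logic attached.
; Disconnected nodes would register each joining lobby player controller and trigger its old menu creation and initial setup.
; A second disconnected chain would rebuild the profile list from connected controllers and send it to each one to update player names.
; The construction script is empty.
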(event Custom|UpdateLobby%20Old
  (params (UpdatePlayerNames :type Boolean)))

(event EventHandleStartingNewPlayer
  (params (NewPlayer :type Player%20Controller%20Object%20Reference)))

(fn ConstructionScript)