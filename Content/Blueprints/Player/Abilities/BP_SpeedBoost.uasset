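; Speed boost player ability that temporarily doubles the walk speed of the player it is applied to.
; On activation it stores that player and multiplies the Character Movement component's MaxWalkSpeed by two.
; On expiry, if the player is still valid, it sets MaxWalkSpeed to half of GetMaxSpeed, which depends on the current movement mode, rather than restoring a saved value.
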(event EventOnAbilityActivated
  (params (PlayerToApplyPowerup :type Actor%20Object%20Reference))
  ;[1 1 1] Activated
  (bind _output_get (Variables|Default|SetPowerupAppliedTo PlayerToApplyPowerup))
  (Variables|/Script/Engine.CharacterMovementComponent|SetMaxWalkSpeed (Actor|GetComponentbyClass _output_get "/Script/Engine.CharacterMovementComponent") (* (Variables|/Script/Engine.CharacterMovementComponent|GetMaxWalkSpeed (Actor|GetComponentbyClass _output_get "/Script/Engine.CharacterMovementComponent")) 2.0)))

(event EventOnAbilityExpired
  (bind _powerupappliedto (Variables|Default|GetPowerupAppliedTo))
  (bind _returnvalue (Actor|GetComponentbyClass _powerupappliedto "/Script/Engine.CharacterMovementComponent"))
  ;[1 1 1] Expired
  (Utilities|IsValid _powerupappliedto
    (:Is%20Valid
      (Variables|/Script/Engine.CharacterMovementComponent|SetMaxWalkSpeed _returnvalue (/ (Class|MovementComponent|GetMaxSpeed _returnvalue) 2.0)))))

(fn ConstructionScript)